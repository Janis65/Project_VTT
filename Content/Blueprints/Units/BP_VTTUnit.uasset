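; Tabletop RPG unit with a D&D-style character sheet, acting in turn-based combat.
; BeginPlay builds its action list from fixed spells and abilities plus an attack per equipped weapon.
; MoveUnit drives AI movement, limited in combat to the active unit; Tick deducts distance traveled from speed, which StartUnitTurn refills along with actions.
; It also resolves damage through temporary HP, rolls d20 saving throws and shows a hover target indicator.
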(event `self.ReceiveBeginPlay`
  (bind _characteractions (`self.CharacterActions`))
  (bind _returnvalue (`|GenericCreateObject` "/Game/Blueprints/Attacks_Spells_Abilities/BP_WhirlwindSlash.BP_WhirlwindSlash_C"))
  (`KismetArrayLibrary.Array_Add` (`self.CharacterActions`) _returnvalue)
  (bind _returnvalue_2 (`|GenericCreateObject` "/Game/Blueprints/Attacks_Spells_Abilities/BP_Spell_FireBall.BP_Spell_FireBall_C"))
  (`KismetArrayLibrary.Array_Add` (`self.CharacterActions`) _returnvalue_2)
  (bind _returnvalue_3 (`|GenericCreateObject` "/Game/Blueprints/Attacks_Spells_Abilities/BP_Spell_FireBolt.BP_Spell_FireBolt_C"))
  (`KismetArrayLibrary.Array_Add` (`self.CharacterActions`) _returnvalue_3)
  (bind _returnvalue_4 (`|GenericCreateObject` "/Game/Blueprints/Attacks_Spells_Abilities/BP_DashAction.BP_DashAction_C"))
  (`KismetArrayLibrary.Array_Add` (`self.CharacterActions`) _returnvalue_4)
  (for _array_element (`self.EquipedWeapon`)
    (bind _returnvalue_5 (`|GenericCreateObject` _array_element "/Game/Blueprints/Attacks_Spells_Abilities/BP_WeaponAttackAction.BP_WeaponAttackAction_C"))
    (set `/Game/Blueprints/Attacks_Spells_Abilities/BP_WeaponAttackAction.WeaponData` _array_element _returnvalue_5)
    (`KismetArrayLibrary.Array_Add` _characteractions _returnvalue_5)
    (for _array_element_2 _characteractions
      (set `/Game/Blueprints/Attacks_Spells_Abilities/BP_BaseAction.Caster` self _array_element_2)
      (`/Game/Blueprints/Attacks_Spells_Abilities/BP_BaseAction.SetVariablesOnSpawn` _array_element_2))))

(event `self.ReceiveActorBeginCursorOver`
  (if (not (`self.IsSelectedAsActiveUnit`))
    (`SceneComponent.SetVisibility` (`self.TargetSelectionIndicator`) true false)))

(event `self.ReceiveActorEndCursorOver`
  (if (not (`self.IsSelectedAsTarget`))
    (`SceneComponent.SetVisibility` (`self.TargetSelectionIndicator`) false false)))

(event `self.ReceiveTick`
  (params (DeltaSeconds :type "Float (single-precision)"))
  (`self.CalculatingDistanceTraveledInCombat`))

(event `Move Unit`
  (params (Destination :type "Vector Structure") (Target :type "/Game/Blueprints/Units/BP_VTTUnit Object Reference") (MoveAcceptRadius :type "Float (double-precision)"))
  ; Checking if combat is active and if it is, checking if selected unit is the one with active turn
  (bind _asbp_vttgame_mode (cast `/Game/Blueprints/Core/BP_VTTGameMode` (`GameplayStatics.GetGameMode`)))
  (bind _currentcombatmanager (`/Game/Blueprints/Core/BP_VTTGameMode.CurrentCombatManager` _asbp_vttgame_mode))
  (if (`/Game/Blueprints/Core/BP_CombatManager.CombatStateActive` _currentcombatmanager)
    (if (== self (`/Game/Blueprints/Core/BP_CombatManager.ActiveUnit` _currentcombatmanager))
      ; Checking what move speed unit has in combat (Experimental)
      (if (>= (`CharacterSheet.CurrentSpeed` (`self.CharacterSheet`)) 0.0)
        (set `self.IsMoving` true)
        ; Moving Unit Out Of Combat (Experimental)
        (`|AIMoveTo` self Destination Target MoveAcceptRadius :!label _label
          (:`OnSuccess`
            (set `self.IsMoving` false)))
        (else
          (`KismetSystemLibrary.PrintString` "Brak ruchu"))))
    (else
      (goto _label))))

(fn `CalculatingDistanceTraveledInCombat`
  (bind _charactersheet (`self.CharacterSheet`))
  (bind _currentspeed (`CharacterSheet.CurrentSpeed` _charactersheet))
  (if (`self.IsMoving`)
    (set `CharacterSheet.CurrentSpeed` (- _currentspeed (`KismetMathLibrary.Vector_Distance` (`self.K2_GetActorLocation`) (`self.LastFrameLocation`))) _charactersheet)
    (set `self.LastFrameLocation` (`self.K2_GetActorLocation`))
    (if (<= _currentspeed 0.0)
      (`MovementComponent.StopMovementImmediately` (`self.CharacterMovement`))
      (set `self.IsMoving` false))))

(fn `EndUnitTurn`)

(fn `MakeSavingThrow`
  (params (SaveDC :type Integer) (SaveType :type "/Game/Data/E_ScalingAttribute Enum" :default "NewEnumerator0"))
  (returns (SaveResult :type Integer) (IsSaved :type Boolean))
  (locals (SaveValue :type Integer))
  (bind _returnvalue (`KismetMathLibrary.RandomIntegerInRange` 1 20))
  (bind _savevalue (`local.SaveValue`))
  (bind (_stats_strength _stats_dexterity _stats_constitution _stats_intelligence _stats_wisdom _stats_charisma) (break `AbilityScores` (`CharacterSheet.Stats` (`self.CharacterSheet`))))
  (switch `/Game/Data/E_ScalingAttribute` SaveType
    (:`NewEnumerator0`
      (set `local.SaveValue` (+ _returnvalue (- (/ _stats_strength 2) 5))))
    (:`NewEnumerator1`
      (set `local.SaveValue` (+ _returnvalue (- (/ _stats_dexterity 2) 5))))
    (:`NewEnumerator2`
      (set `local.SaveValue` (+ _returnvalue (- (/ _stats_constitution 2) 5))))
    (:`NewEnumerator3`
      (set `local.SaveValue` (+ _returnvalue (- (/ _stats_intelligence 2) 5))))
    (:`NewEnumerator4`
      (set `local.SaveValue` (+ _returnvalue (- (/ _stats_wisdom 2) 5))))
    (:`NewEnumerator5`
      (set `local.SaveValue` (+ _returnvalue (- (/ _stats_charisma 2) 5))))
    (:`NewEnumerator6`
      (set `local.SaveValue` _returnvalue)))
  (`/Engine/EditorBlueprintResources/StandardMacros.CompareInt` _savevalue SaveDC
    (:`>`
      _)
    (:`==`
      _)
    (:`<`
      (return _savevalue false)))
  (return _savevalue true))

(fn `StartUnitTurn`
  (bind _charactersheet (`self.CharacterSheet`))
  (bind (_actions_maxactions _actions_currentactions _actions_maxbonusactions _actions_currentbonusactions _actions_maxreactions) (break `Actions` (`CharacterSheet.Actions` _charactersheet)))
  (set `self.LastFrameLocation` (`self.K2_GetActorLocation`))
  (set `CharacterSheet.CurrentSpeed` (`CharacterSheet.MaxSpeed` _charactersheet) _charactersheet)
  (set `CharacterSheet.Actions` (make `Actions` _actions_maxactions _actions_maxactions _actions_maxbonusactions _actions_maxbonusactions _actions_maxreactions _actions_maxreactions) _charactersheet))

(fn `TakeDamage`
  (params (Damage :type "Map of /Game/Data/E_DamageType Enum to Integer"))
  (bind _temporaryhp (`CharacterSheet.TemporaryHP` (`self.CharacterSheet`)))
  (bind (_keypin _valuepin) (`|MapForEach` Damage)
    (:`then`
      (bind _returnvalue (`KismetMathLibrary.Min` _valuepin _temporaryhp))
      (bind _output_get (set `CharacterSheet.CurrentHP` (- (`CharacterSheet.CurrentHP` (`self.CharacterSheet`)) (- _valuepin _returnvalue)) (`self.CharacterSheet`)))
      (set `CharacterSheet.TemporaryHP` (- _temporaryhp _returnvalue) (`self.CharacterSheet`))
      (if (<= _output_get 0)
        (set `self.IsDead` true)))))

(fn `UserConstructionScript`)