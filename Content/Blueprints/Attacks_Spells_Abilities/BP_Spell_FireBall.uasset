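; Fireball spell action that deals area damage, with a saving throw for half damage.
; On spawn it copies range, icon and area shape from SpellData.
; ExecuteAction rolls damage only when the Damage map is empty, caches halved values in SaveDamage, then applies either map per target based on a save against the caster's spell DC.
; ConsumeResources clears Damage, so the next execution rolls again.
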(event `self.ExecuteAction`
  (params (Target :type "/Game/Blueprints/Units/BP_VTTUnit Object Reference"))
  (if (<= (`BlueprintMapLibrary.Map_Length` (`self.Damage`)) 0)
    (bind _damage (`/Game/Blueprints/Attacks_Spells_Abilities/Spells/DA_Spell.CalculateDamageRoll` (`self.SpellData`) false))
    (bind _output_get (set `self.Damage` _damage))
    (bind (_keypin _valuepin) (`|MapForEach` _output_get)
      (:`then`
        (`BlueprintMapLibrary.Map_Add` (`self.SaveDamage`) _keypin (/ _valuepin 2)))
      (:`CompletedPin`
        (bind _output_get_2 (set `self.AttackTarget` Target :!label _label))
        (bind (_saveresult _issaved) (`/Game/Blueprints/Units/BP_VTTUnit.MakeSavingThrow` _output_get_2 (`CharacterSheet.SpellSaveDC` (`/Game/Blueprints/Units/BP_VTTUnit.CharacterSheet` (`self.Caster`))) "NewEnumerator1"))
        (if _issaved
          (`/Game/Blueprints/Units/BP_VTTUnit.TakeDamage` (`self.AttackTarget`) (`self.SaveDamage`))
          (else
            (`/Game/Blueprints/Units/BP_VTTUnit.TakeDamage` (`self.AttackTarget`) (`self.Damage`))))))
    (else
      (goto _label))))

(event `self.SetVariablesOnSpawn`
  (bind _spelldata (`self.SpellData`))
  ; Set Action Variables On Spawn
  (set `self.ActionRange` (`/Game/Blueprints/Attacks_Spells_Abilities/Spells/DA_Spell.MaxRange` _spelldata))
  (set `self.Icon` (`/Game/Blueprints/Attacks_Spells_Abilities/Spells/DA_Spell.Icon` _spelldata))
  (set `self.AreaType` (`/Game/Blueprints/Attacks_Spells_Abilities/Spells/DA_Spell.AreaType` _spelldata))
  (set `self.AreaDimension` (`/Game/Blueprints/Attacks_Spells_Abilities/Spells/DA_Spell.AreaDimension` _spelldata)))

(event `self.Consume Resources`
  (`BlueprintMapLibrary.Map_Clear` (`self.Damage`)))