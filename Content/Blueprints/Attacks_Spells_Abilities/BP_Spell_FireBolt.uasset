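; Fire Bolt spell action that makes an attack roll against a target's Armor Class and applies damage on a hit.
; ExecuteAction compares caster-to-target distance with the spell's max range to pick the roll's advantage type.
; SpellData handles the attack and crit-aware damage rolls, and supplies range and icon on spawn.
; Results print as debug strings, and the ConsumeAction calls are unconnected.
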(event `self.ExecuteAction`
  (params (Target :type "/Game/Blueprints/Units/BP_VTTUnit Object Reference"))
  (bind _spelldata (`self.SpellData`))
  (bind _spelldata_2 (`self.SpellData`))
  (set `self.AttackTarget` Target)
  ; Making Attack Roll And If It Hits Damage Roll
  (if (> (`KismetMathLibrary.Vector_Distance` (`Actor.K2_GetActorLocation` (`self.Caster`)) (`Actor.K2_GetActorLocation` (`self.AttackTarget`))) (`/Game/Blueprints/Attacks_Spells_Abilities/Spells/DA_Spell.MaxRange` (`self.SpellData`)))
    (bind (_ishit _iscrit _attackroll) (`/Game/Blueprints/Attacks_Spells_Abilities/Spells/DA_Spell.MakeAttackRoll` _spelldata (`CharacterSheet.ArmorClass` (`/Game/Blueprints/Units/BP_VTTUnit.CharacterSheet` (`self.AttackTarget`))) "NewEnumerator2"))
    (if _ishit
      (`KismetSystemLibrary.PrintString` null (`KismetStringLibrary.Conv_IntToString` _attackroll))
      (bind _damage (`/Game/Blueprints/Attacks_Spells_Abilities/Spells/DA_Spell.CalculateDamageRoll` _spelldata _iscrit))
      (`/Game/Blueprints/Units/BP_VTTUnit.TakeDamage` (`self.AttackTarget`) _damage)
      (else
        (`KismetSystemLibrary.PrintString` null "Miss!!")))
    (else
      (bind (_ishit_2 _iscrit_2 _attackroll_2) (`/Game/Blueprints/Attacks_Spells_Abilities/Spells/DA_Spell.MakeAttackRoll` _spelldata_2 (`CharacterSheet.ArmorClass` (`/Game/Blueprints/Units/BP_VTTUnit.CharacterSheet` (`self.AttackTarget`))) "NewEnumerator1"))
      (if _ishit_2
        (`KismetSystemLibrary.PrintString` null (`KismetStringLibrary.Conv_IntToString` _attackroll_2))
        (bind _damage_2 (`/Game/Blueprints/Attacks_Spells_Abilities/Spells/DA_Spell.CalculateDamageRoll` _spelldata_2 _iscrit_2))
        (`/Game/Blueprints/Units/BP_VTTUnit.TakeDamage` (`self.AttackTarget`) _damage_2)
        (else
          (`KismetSystemLibrary.PrintString` null "Miss!!"))))))

(event `self.SetVariablesOnSpawn`
  (bind _spelldata (`self.SpellData`))
  ; Set Action Variables On Spawn
  (set `self.ActionRange` (`/Game/Blueprints/Attacks_Spells_Abilities/Spells/DA_Spell.MaxRange` _spelldata))
  (set `self.Icon` (`/Game/Blueprints/Attacks_Spells_Abilities/Spells/DA_Spell.Icon` _spelldata)))