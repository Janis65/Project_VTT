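; Ray of Frost cantrip action that makes an attack roll against each target's armor class, deals damage on a hit and slows the victim.
; Targets beyond the spell's max range are rolled with a different advantage type.
; A hit cuts the target's max speed and binds EndEffect to the caster's turn start, which restores speed on the last stored target and unbinds.
; The action is consumed after all targets resolve.
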(event `self.ExecuteAction`
  (params (Targets :type "Array of /Game/Blueprints/Units/BP_VTTUnit Object Reference (by ref)"))
  (bind _spelldata (`self.SpellData`))
  (bind _spelldata_2 (`self.SpellData`))
  (bind _attacktarget (`self.AttackTarget`))
  (bind _charactersheet (`/Game/Blueprints/Units/BP_VTTUnit.CharacterSheet` _attacktarget))
  (for _array_element Targets
    (set `self.AttackTarget` _array_element)
    ; Making Attack Roll And If It Hits Damage Roll
    (if (> (`KismetMathLibrary.Vector_Distance` (`Actor.K2_GetActorLocation` (`self.Caster`)) (`Actor.K2_GetActorLocation` (`self.AttackTarget`))) (`/Game/Blueprints/Attacks_Spells_Abilities/Spells/Spell_DA/DA_Spell.MaxRange` (`self.SpellData`)))
      (bind (_ishit _iscrit _attackroll) (`/Game/Blueprints/Attacks_Spells_Abilities/Spells/Spell_DA/DA_Spell.MakeAttackRoll` _spelldata (`CharacterSheet.ArmorClass` (`/Game/Blueprints/Units/BP_VTTUnit.CharacterSheet` (`self.AttackTarget`))) "NewEnumerator2"))
      (if _ishit
        (`KismetSystemLibrary.PrintString` null (`KismetStringLibrary.Conv_IntToString` _attackroll))
        (bind _damage (`/Game/Blueprints/Attacks_Spells_Abilities/Spells/Spell_DA/DA_Spell.CalculateDamageRoll` _spelldata _iscrit))
        (`/Game/Blueprints/Units/BP_VTTUnit.TakeDamage` (`self.AttackTarget`) _damage)
        (set `CharacterSheet.MaxSpeed` (- (`CharacterSheet.MaxSpeed` _charactersheet) 300.0) _charactersheet :!label _label)
        (add `/Game/Blueprints/Units/BP_VTTUnit.UnitTurnStart` (`self.Caster`) (delegate `EndEffect`))
        (else
          (`KismetSystemLibrary.PrintString` null "Miss!!")))
      (else
        (bind (_ishit_2 _iscrit_2 _attackroll_2) (`/Game/Blueprints/Attacks_Spells_Abilities/Spells/Spell_DA/DA_Spell.MakeAttackRoll` _spelldata_2 (`CharacterSheet.ArmorClass` (`/Game/Blueprints/Units/BP_VTTUnit.CharacterSheet` (`self.AttackTarget`))) "NewEnumerator1"))
        (if _ishit_2
          (`KismetSystemLibrary.PrintString` null (`KismetStringLibrary.Conv_IntToString` _attackroll_2))
          (bind _damage_2 (`/Game/Blueprints/Attacks_Spells_Abilities/Spells/Spell_DA/DA_Spell.CalculateDamageRoll` _spelldata_2 _iscrit_2))
          (`/Game/Blueprints/Units/BP_VTTUnit.TakeDamage` _attacktarget _damage_2)
          (goto _label)
          (else
            (`KismetSystemLibrary.PrintString` null "Miss!!"))))))
  (`self.ConsumeAction` true))

(event `EndEffect`
  (bind _charactersheet (`/Game/Blueprints/Units/BP_VTTUnit.CharacterSheet` (`self.AttackTarget`)))
  (set `CharacterSheet.MaxSpeed` (+ (`CharacterSheet.MaxSpeed` _charactersheet) 300.0) _charactersheet)
  (remove `/Game/Blueprints/Units/BP_VTTUnit.UnitTurnStart` (`self.Caster`) (delegate `EndEffect`)))