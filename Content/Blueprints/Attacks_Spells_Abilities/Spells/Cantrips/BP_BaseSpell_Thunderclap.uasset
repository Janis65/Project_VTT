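; Thunderclap cantrip spell Blueprint that damages targets in range unless they resist with a saving throw.
; On execute, it rolls damage once from its spell data for all targets.
; Each target makes a Constitution save against the caster's spell save DC and takes the full roll only on a failure.
; After the loop, the action is consumed.
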(event `self.ExecuteAction`
  (params (Targets :type "Array of /Game/Blueprints/Units/BP_VTTUnit Object Reference (by ref)"))
  ; Make Saving Throw For Each Target In Range And If It Hits Damage Roll
  (`|ExecutionSequence`
    (:`then_0`
      (bind _damage (`/Game/Blueprints/Attacks_Spells_Abilities/Spells/Spell_DA/DA_Spell.CalculateDamageRoll` (`self.SpellData`) false)))
    (:`then_1`
      (for _array_element Targets
        (bind _output_get (set `self.AttackTarget` _array_element))
        (bind (_saveresult _issaved) (`/Game/Blueprints/Units/BP_VTTUnit.MakeSavingThrow` _output_get (`CharacterSheet.SpellSaveDC` (`/Game/Blueprints/Units/BP_VTTUnit.CharacterSheet` (`self.Caster`))) "Constitution"))
        (if (not _issaved)
          (`/Game/Blueprints/Units/BP_VTTUnit.TakeDamage` (`self.AttackTarget`) _damage)))
      (`self.ConsumeAction` true))))