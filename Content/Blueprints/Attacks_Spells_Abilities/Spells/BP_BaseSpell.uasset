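; Base spell Blueprint that sets up a spell action from its data and handles its slot cost for the caster.
; SetVariablesonSpawn copies range, icon, area type and area dimension from SpellData into the action's variables.
; ConsumeResources switches on the spell's level and decrements the matching current slot count on the caster's character sheet, covering levels one to five with no availability check.
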(event `self.SetVariablesOnSpawn`
  (bind _spelldata (`self.SpellData`))
  ; Set Action Variables On Spawn
  (set `self.ActionRange` (`/Game/Blueprints/Attacks_Spells_Abilities/Spells/Spell_DA/DA_Spell.MaxRange` _spelldata))
  (set `self.Icon` (`/Game/Blueprints/Attacks_Spells_Abilities/Spells/Spell_DA/DA_Spell.Icon` _spelldata))
  (set `self.AreaType` (`/Game/Blueprints/Attacks_Spells_Abilities/Spells/Spell_DA/DA_Spell.AreaType` _spelldata))
  (set `self.AreaDimension` (`/Game/Blueprints/Attacks_Spells_Abilities/Spells/Spell_DA/DA_Spell.AreaDimension` _spelldata)))

(event `self.Consume Resources`
  (bind (_spellslots_level1_max _spellslots_level1_current _spellslots_level2_max _spellslots_level2_current _spellslots_level3_max _spellslots_level3_current _spellslots_level4_max _spellslots_level4_current _spellslots_level5_max _spellslots_level5_current) (break `SpellSlots` (`CharacterSheet.SpellSlots` (`/Game/Blueprints/Units/BP_VTTUnit.CharacterSheet` (`self.Caster`)))))
  (switch `int` (`/Game/Blueprints/Attacks_Spells_Abilities/Spells/Spell_DA/DA_Spell.SpellLevel` (`self.SpellData`))
    (:`1`
      (`/Engine/EditorBlueprintResources/StandardMacros.DecrementInt` _spellslots_level1_current))
    (:`2`
      (`/Engine/EditorBlueprintResources/StandardMacros.DecrementInt` _spellslots_level2_current))
    (:`3`
      (`/Engine/EditorBlueprintResources/StandardMacros.DecrementInt` _spellslots_level3_current))
    (:`4`
      (`/Engine/EditorBlueprintResources/StandardMacros.DecrementInt` _spellslots_level4_current))
    (:`5`
      (`/Engine/EditorBlueprintResources/StandardMacros.DecrementInt` _spellslots_level5_current))))