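; Shield is a 1st-level spell Blueprint that temporarily raises the caster's Armor Class by 5.
; On execution it adds the bonus to the caster's character sheet, consumes the action and resources, and binds an end callback to the caster's unit turn start event.
; When that event fires, the callback subtracts the same bonus and unbinds itself.
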(event `self.ExecuteAction`
  (params (Targets :type "Array of /Game/Blueprints/Units/BP_VTTUnit Object Reference (by ref)"))
  (bind _caster (`self.Caster`))
  (bind _charactersheet (`/Game/Blueprints/Units/BP_VTTUnit.CharacterSheet` _caster))
  (set `CharacterSheet.ArmorClass` (+ (`CharacterSheet.ArmorClass` _charactersheet) 5) _charactersheet)
  (`self.ConsumeAction` true)
  (`self.Consume Resources`)
  (add `/Game/Blueprints/Units/BP_VTTUnit.UnitTurnStart` _caster (delegate `EndEffect`)))

(event `EndEffect`
  (bind _caster (`self.Caster`))
  (bind _charactersheet (`/Game/Blueprints/Units/BP_VTTUnit.CharacterSheet` _caster))
  (set `CharacterSheet.ArmorClass` (- (`CharacterSheet.ArmorClass` _charactersheet) 5) _charactersheet)
  (remove `/Game/Blueprints/Units/BP_VTTUnit.UnitTurnStart` _caster (delegate `EndEffect`)))