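; BP_WhirlwindSlash is an attack action that resolves a weapon strike against a single target.
; When executed, it makes an attack roll through WeaponData against the target's Armor Class, then applies rolled damage on a hit, accounting for crits.
; The attack roll and misses are printed as debug strings.
; On spawn it takes its range from the weapon's optimal range; its ConsumeAction call is never run.
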(event `self.ExecuteAction`
  (params (Target :type "/Game/Blueprints/Units/BP_VTTUnit Object Reference"))
  (bind _weapondata (`self.WeaponData`))
  (set `self.AttackTarget` Target)
  ; Making Attack Roll And If It Hits Damage Roll
  (bind (_ishit _iscrit _attackroll) (`/Game/Blueprints/Attacks_Spells_Abilities/Items/DA_Weapon.MakeAttackRoll` _weapondata (`CharacterSheet.ArmorClass` (`/Game/Blueprints/Units/BP_VTTUnit.CharacterSheet` (`self.AttackTarget`))) "NewEnumerator1"))
  (if _ishit
    (`KismetSystemLibrary.PrintString` null (`KismetStringLibrary.Conv_IntToString` _attackroll))
    (bind _damage (`/Game/Blueprints/Attacks_Spells_Abilities/Items/DA_Weapon.CalculateDamageRoll` _weapondata _iscrit))
    (`/Game/Blueprints/Units/BP_VTTUnit.TakeDamage` (`self.AttackTarget`) _damage)
    (else
      (`KismetSystemLibrary.PrintString` null "Miss!!"))))

(event `self.SetVariablesOnSpawn`
  ; Set Action Variables On Spawn
  (set `self.ActionRange` (`/Game/Blueprints/Attacks_Spells_Abilities/Items/DA_Weapon.OptimalRange` (`self.WeaponData`))))