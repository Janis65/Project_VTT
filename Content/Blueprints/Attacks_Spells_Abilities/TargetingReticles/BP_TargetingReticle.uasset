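; BP_TargetingReticle is a targeting reticle actor that tracks which VTT units lie inside its area, likely for attacks and spells.
; On overlap begin, it shows the unit's TargetSelectionIndicator and adds the unit to OverlappingTargets.
; On overlap end, it hides the indicator and removes the unit, while other actor types are ignored.
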(event `self.ReceiveTick`
  (params (DeltaSeconds :type "Float (single-precision)")))

(event `self.ReceiveActorBeginOverlap`
  (params (OtherActor :type "Actor Object Reference"))
  (bind _asbp_vttunit (cast `/Game/Blueprints/Units/BP_VTTUnit` OtherActor))
  (`SceneComponent.SetVisibility` (`/Game/Blueprints/Units/BP_VTTUnit.TargetSelectionIndicator` _asbp_vttunit) true false)
  (`KismetArrayLibrary.Array_Add` (`self.OverlappingTargets`) _asbp_vttunit))

(event `self.ReceiveActorEndOverlap`
  (params (OtherActor :type "Actor Object Reference"))
  (bind _asbp_vttunit (cast `/Game/Blueprints/Units/BP_VTTUnit` OtherActor))
  (`SceneComponent.SetVisibility` (`/Game/Blueprints/Units/BP_VTTUnit.TargetSelectionIndicator` _asbp_vttunit) false false)
  (`KismetArrayLibrary.Array_RemoveItem` (`self.OverlappingTargets`) _asbp_vttunit))

(fn `UserConstructionScript`)