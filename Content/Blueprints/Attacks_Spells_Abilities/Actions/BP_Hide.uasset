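; BP_Hide is a Hide action that makes a d20-style Stealth check for its caster.
; On ExecuteAction it reads the caster's Stealth skill modifier, adds it to a random 1–20 roll, and prints the breakdown as a string.
; It then calls ConsumeAction; the result is only printed, with no hidden state applied or comparison against a target.
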(event `self.ExecuteAction`
  (params (Targets :type "Array of /Game/Blueprints/Units/BP_VTTUnit Object Reference (by ref)"))
  (bind _returnvalue (`KismetMathLibrary.RandomIntegerInRange` 1 20))
  (bind _modifier (`/Game/Blueprints/Units/BP_VTTUnit.GetSkillModifier` (`self.Caster`) "Stealth"))
  (`KismetSystemLibrary.PrintString` null (`KismetStringLibrary.Concat_StrStr` (`|GetEnumeratorNameAsString` (enumliteral `ESkillType` "Stealth")) ":" (`KismetStringLibrary.Conv_IntToString` _returnvalue) "+" (`KismetStringLibrary.Conv_IntToString` _modifier) "=" (`KismetStringLibrary.Conv_IntToString` (+ _returnvalue _modifier))))
  (`self.ConsumeAction` true))