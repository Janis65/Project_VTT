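; BP_ActionSurge is the Warrior's Action Surge ability, which grants the caster an extra action.
; Executing it while uses remain increments the current action count on the caster's character sheet and spends one use.
; On spawn setup it binds RechargeUses to the caster's short and long rest finished events, so either rest restores uses to the maximum.
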(event `self.ExecuteAction`
  (params (Targets :type "Array of /Game/Blueprints/Units/BP_VTTUnit Object Reference (by ref)"))
  (bind (_actions_maxactions _actions_currentactions) (break `Actions` (`CharacterSheet.Actions` (`/Game/Blueprints/Units/BP_VTTUnit.CharacterSheet` (`self.Caster`)))))
  (if (> (`self.CurrentUses`) 0)
    (`/Engine/EditorBlueprintResources/StandardMacros.IncrementInt` _actions_currentactions
      (:`  `
        (`/Engine/EditorBlueprintResources/StandardMacros.DecrementInt` (`self.CurrentUses`))))))

(event `self.SetVariablesOnSpawn`
  (bind _caster (`self.Caster`))
  (add `/Game/Blueprints/Units/BP_VTTUnit.ShortRestFinished` _caster (delegate `self.RechargeUses`))
  (add `/Game/Blueprints/Units/BP_VTTUnit.LongRestFinished` _caster (delegate `self.RechargeUses`)))

(event `self.RechargeUses`
  (set `self.CurrentUses` (`self.MaxUses`)))