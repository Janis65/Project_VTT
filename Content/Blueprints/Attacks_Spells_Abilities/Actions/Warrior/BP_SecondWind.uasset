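; Second Wind is a Fighter ability action that heals the caster by a d10 roll plus their Fighter class level.
; Executing it spends one use if any remain and clamps the new HP to the character sheet's maximum.
; On spawn it binds to the caster's short and long rest events, which restore all uses.
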(event `self.ExecuteAction`
  (params (Target :type "/Game/Blueprints/Units/BP_VTTUnit Object Reference"))
  (bind _caster (`self.Caster`))
  (bind _charactersheet (`/Game/Blueprints/Units/BP_VTTUnit.CharacterSheet` _caster))
  (if (> (`self.CurrentUses`) 0)
    (set `CharacterSheet.CurrentHP` (`KismetMathLibrary.Clamp` (+ (`CharacterSheet.CurrentHP` _charactersheet) (+ (`KismetMathLibrary.RandomIntegerInRange` 1 10) (`BlueprintMapLibrary.Map_Find` (`/Game/Blueprints/Units/BP_VTTUnit.CharacterClasses` _caster) "/Game/Blueprints/Classes/DA_Class_Fighter.DA_Class_Fighter"))) 0 (`CharacterSheet.MaxHP` _charactersheet)) _charactersheet)
    (`/Engine/EditorBlueprintResources/StandardMacros.DecrementInt` (`self.CurrentUses`))))

(event `self.SetVariablesOnSpawn`
  (bind _caster (`self.Caster`))
  (add `/Game/Blueprints/Units/BP_VTTUnit.ShortRestFinished` _caster (delegate `self.RechargeUses`))
  (add `/Game/Blueprints/Units/BP_VTTUnit.LongRestFinished` _caster (delegate `self.RechargeUses`)))

(event `self.RechargeUses`
  (set `self.CurrentUses` (`self.MaxUses`)))