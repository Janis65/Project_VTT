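; BP_SneakAttack is a Rogue action meant to roll Sneak Attack damage against each target.
; ExecuteAction resets the total per target, then sums d6 rolls, with the count taken from GrantedClassResources in the class's LevelUpData.
; The class and level come from an index lookup on the caster's CharacterClasses, using the Rogue entry's value as the index.
; The rolled total is unused and the TakeDamage call is unconnected, so no damage is applied.
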(event `self.ExecuteAction`
  (params (Targets :type "Array of /Game/Blueprints/Units/BP_VTTUnit Object Reference (by ref)"))
  (bind _characterclasses (`/Game/Blueprints/Units/BP_VTTUnit.CharacterClasses` (`self.Caster`)))
  (bind (_key _value) (`BlueprintMapLibrary.Map_GetKeyValueByIndex` _characterclasses (`BlueprintMapLibrary.Map_Find` _characterclasses "/Game/Blueprints/Classes/DA_Class_Rogue.DA_Class_Rogue")))
  (for _array_element Targets
    (set `self.SneakAttackDamage` 0)
    (for _ (range 1 (+ (`.GrantedClassResources_15_FB88ABF248475C5E5452FE91FFDF6743` (break `/Game/Data/Classes/S_LevelUpProgression` (`BlueprintMapLibrary.Map_Find` (`/Game/Data/Classes/DA_CharacterClass.LevelUpData` _key) _value))) 1))
      (set `self.SneakAttackDamage` (+ (`KismetMathLibrary.RandomIntegerInRange` 1 6) (`self.SneakAttackDamage`))))))