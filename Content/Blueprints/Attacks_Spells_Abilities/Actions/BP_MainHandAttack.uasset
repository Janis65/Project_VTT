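; Action Blueprint for a main-hand weapon attack in a tabletop-style combat system with armor class, crits and multiple attacks per action.
; On execute it consumes an action and refills attacks when none remain, then handles each target, using AI movement if out of weapon range.
; The weapon rolls attack and damage; misses spawn Niagara "Miss!!" text, and each attack decrements AttacksLeft.
; Shield-spell reaction hooks are unwired, and both continue events are empty.
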(event `self.SetVariablesOnSpawn`
  ; Set Action Variables On Spawn
  (set `self.ActionRange` (`/Game/Blueprints/Items/DA_Weapon.OptimalRange` (`/Game/Blueprints/Units/BP_VTTUnit.MainHandWeapon` (`self.Caster`)))))

(event `self.ContinueAction2`)

(event `self.ContinueAction1`
  ; Making Attack Roll And If It Hits Damage Roll
)

(event `self.ExecuteAction`
  (params (Targets :type "Array of /Game/Blueprints/Units/BP_VTTUnit Object Reference (by ref)"))
  (bind _caster (`self.Caster`))
  (bind _caster_2 (`self.Caster`))
  (bind _attacktarget (`self.AttackTarget`))
  (bind _caster_3 (`self.Caster`))
  (bind _mainhandweapon (`/Game/Blueprints/Units/BP_VTTUnit.MainHandWeapon` (`self.Caster`)))
  (bind _mainhandweapon_2 (`/Game/Blueprints/Units/BP_VTTUnit.MainHandWeapon` _caster))
  ; Checking If Attacker Is In Distance To Attack And If Not Moving To It
  (if (<= (`/Game/Blueprints/Units/BP_VTTUnit.AttacksLeft` _caster_3) 0)
    (`self.ConsumeAction` true)
    (set `/Game/Blueprints/Units/BP_VTTUnit.AttacksLeft` (`/Game/Blueprints/Units/BP_VTTUnit.MaxAttacksPerAction` _caster_3) _caster_3))
  (for _array_element Targets
    (set `self.AttackTarget` _array_element)
    (if (> (`KismetMathLibrary.Vector_Distance` (`Actor.K2_GetActorLocation` (`self.Caster`)) (`Actor.K2_GetActorLocation` (`self.AttackTarget`))) (`/Game/Blueprints/Items/DA_Weapon.OptimalRange` _mainhandweapon))
      (set `/Game/Blueprints/Units/BP_VTTUnit.IsMoving` true _caster_2)
      (`|AIMoveTo` _caster_2 _caster_2 (0.0 0.0 0.0) (`self.AttackTarget`) (`/Game/Blueprints/Items/DA_Weapon.OptimalRange` _mainhandweapon)
        (:`OnSuccess`
          _)))
    ; Making Attack Roll And If It Hits Damage Roll
    (bind (_ishit _iscrit _attackroll) (`/Game/Blueprints/Items/DA_Weapon.MakeAttackRoll` _mainhandweapon_2 (`CharacterSheet.ArmorClass` (`/Game/Blueprints/Units/BP_VTTUnit.CharacterSheet` _attacktarget)) "NewEnumerator1" _caster))
    (if _ishit
      (`KismetSystemLibrary.PrintString` null (`KismetStringLibrary.Conv_IntToString` _attackroll))
      (bind _damage (`/Game/Blueprints/Items/DA_Weapon.CalculateDamageRoll` _mainhandweapon_2 _iscrit _caster))
      (`/Game/Blueprints/Units/BP_VTTUnit.TakeDamage` (`self.AttackTarget`) _damage)
      (else
        (bind _returnvalue (`NiagaraFunctionLibrary.SpawnSystemAtLocation` _attacktarget "/Game/Blueprints/NS_SpawnDamageText.NS_SpawnDamageText" (`Actor.K2_GetActorLocation` _attacktarget)))
        (`NiagaraTextToolkitHelpers.SetNiagaraNTTTextVariable` _returnvalue "Miss!!")))
    (`/Engine/EditorBlueprintResources/StandardMacros.DecrementInt` (`/Game/Blueprints/Units/BP_VTTUnit.AttacksLeft` (`self.Caster`)))))