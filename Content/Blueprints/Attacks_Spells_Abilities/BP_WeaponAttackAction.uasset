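; Weapon attack action for a tabletop-style combat system, rolling the caster's weapon against the target's Armor Class and applying damage on a hit.
; Ranged weapons fire from where they stand, switching advantage type beyond optimal range, while other weapons use AI MoveTo to close in first.
; WeaponData handles attack and crit-aware damage rolls and supplies the action's range and icon.
; Results are only printed, and ConsumeAction is never reached.
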(event `self.ExecuteAction`
  (params (Target :type "/Game/Blueprints/Units/BP_VTTUnit Object Reference"))
  (bind _caster (`self.Caster`))
  (bind _weapondata (`self.WeaponData`))
  (bind _returnvalue (> (`KismetMathLibrary.Vector_Distance` (`Actor.K2_GetActorLocation` (`self.Caster`)) (`Actor.K2_GetActorLocation` (`self.AttackTarget`))) (`/Game/Blueprints/Attacks_Spells_Abilities/Items/DA_Weapon.OptimalRange` (`self.WeaponData`))))
  (set `self.AttackTarget` Target)
  ; Checking If Attacker Is In Distance To Attack And If Not Moving To It
  (`/Game/Blueprints/Attacks_Spells_Abilities/Items/DA_Weapon.IsRanged` (`self.WeaponData`)
    (:`then`
      (if _returnvalue
        ; Making Attack Roll And If It Hits Damage Roll
        (bind (_ishit _iscrit _attackroll) (`/Game/Blueprints/Attacks_Spells_Abilities/Items/DA_Weapon.MakeAttackRoll` _weapondata (`CharacterSheet.ArmorClass` (`/Game/Blueprints/Units/BP_VTTUnit.CharacterSheet` (`self.AttackTarget`))) "NewEnumerator2"))
        (if _ishit
          (`KismetSystemLibrary.PrintString` null (`KismetStringLibrary.Conv_IntToString` _attackroll))
          (bind _damage (`/Game/Blueprints/Attacks_Spells_Abilities/Items/DA_Weapon.CalculateDamageRoll` _weapondata _iscrit))
          (`/Game/Blueprints/Units/BP_VTTUnit.TakeDamage` (`self.AttackTarget`) _damage)
          (else
            (`KismetSystemLibrary.PrintString` null "Miss!!")))
        (else
          (bind (_ishit_2 _iscrit_2 _attackroll_2) (`/Game/Blueprints/Attacks_Spells_Abilities/Items/DA_Weapon.MakeAttackRoll` _weapondata (`CharacterSheet.ArmorClass` (`/Game/Blueprints/Units/BP_VTTUnit.CharacterSheet` (`self.AttackTarget`))) "NewEnumerator1" :!label _label))
          (if _ishit_2
            (`KismetSystemLibrary.PrintString` null (`KismetStringLibrary.Conv_IntToString` _attackroll_2))
            (bind _damage_2 (`/Game/Blueprints/Attacks_Spells_Abilities/Items/DA_Weapon.CalculateDamageRoll` _weapondata _iscrit_2))
            (`/Game/Blueprints/Units/BP_VTTUnit.TakeDamage` (`self.AttackTarget`) _damage_2)
            (else
              (`KismetSystemLibrary.PrintString` null "Miss!!"))))))
    (:`else`
      (if _returnvalue
        (set `/Game/Blueprints/Units/BP_VTTUnit.IsMoving` true _caster)
        (`|AIMoveTo` _caster _caster (0.0 0.0 0.0) (`self.AttackTarget`) (`/Game/Blueprints/Attacks_Spells_Abilities/Items/DA_Weapon.OptimalRange` (`self.WeaponData`))
          (:`OnSuccess`
            (goto _label)))
        (else
          (goto _label))))))

(event `self.SetVariablesOnSpawn`
  (bind _weapondata (`self.WeaponData`))
  ; Set Action Variables On Spawn
  (set `self.ActionRange` (`/Game/Blueprints/Attacks_Spells_Abilities/Items/DA_Weapon.OptimalRange` _weapondata))
  (set `self.Icon` (`/Game/Blueprints/Attacks_Spells_Abilities/Items/DA_Weapon.Icon` _weapondata)))