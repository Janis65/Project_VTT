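; BP_VTTCamera is a player-controlled camera pawn with planar movement, spring-arm zoom and yaw rotation through Enhanced Input actions.
; Every tick a downward visibility trace snaps its height to a fixed offset above the surface below.
; Holding middle mouse enables mouse rotation, hides the cursor and switches to game-only input, while QE rotation works only when it is released.
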(event `self.ReceiveTick`
  (params (DeltaSeconds :type "Float (single-precision)"))
  (bind (_returnvalue_x _returnvalue_y _returnvalue_z) (`KismetMathLibrary.BreakVector` (`self.K2_GetActorLocation`)))
  (bind (_returnvalue_x_2 _returnvalue_y_2 _returnvalue_z_2) (`KismetMathLibrary.BreakVector` (`self.K2_GetActorLocation`)))
  (bind (_returnvalue_x_3 _returnvalue_y_3) (`KismetMathLibrary.BreakVector` (`self.K2_GetActorLocation`)))
  ; Camera Terrain Adaptation
  (bind _outhit (`KismetSystemLibrary.LineTraceSingle` :`Start` (`KismetMathLibrary.MakeVector` _returnvalue_x_2 _returnvalue_y_2 (+ _returnvalue_z_2 (`self.LineTraceStartOffset`))) :`End` (`KismetMathLibrary.MakeVector` _returnvalue_x _returnvalue_y (+ _returnvalue_z -1000.0)) :`TraceChannel` "TraceTypeQuery1" :`DrawDebugType` "ForDuration"))
  (`self.K2_SetActorLocation` (`KismetMathLibrary.MakeVector` _returnvalue_x_3 _returnvalue_y_3 (+ (.z (`.ImpactPoint` (`GameplayStatics.BreakHitResult` _outhit))) (`self.LineTraceStartOffset`)))))

(event `EnhancedInput|/Game/Data/Input/IA_MoveCamera`
  (params (ActionValue :type "Vector2D Structure") (ElapsedSeconds :type "Float (double-precision)") (TriggeredSeconds :type "Float (double-precision)") (InputAction :type "InputAction Object Reference" :default "/Game/Data/Input/IA_MoveCamera.IA_MoveCamera"))
  (bind (_x _y) (`KismetMathLibrary.BreakVector2D` ActionValue))
  ; Camera WASD
  (:`Triggered`
    (`self.AddMovementInput` (`self.GetActorForwardVector`) _x)
    (`self.AddMovementInput` (`self.GetActorRightVector`) _y)))

(event `self.ReceiveBeginPlay`)

(event `EnhancedInput|/Game/Data/Input/IA_ZoomCamera`
  (params (ActionValue :type "Float (double-precision)") (ElapsedSeconds :type "Float (double-precision)") (TriggeredSeconds :type "Float (double-precision)") (InputAction :type "InputAction Object Reference" :default "/Game/Data/Input/IA_ZoomCamera.IA_ZoomCamera"))
  (bind _springarm (`self.SpringArm`))
  ; Camera Zoom
  (:`Triggered`
    (set `SpringArmComponent.TargetArmLength` (`KismetMathLibrary.FClamp` (+ (`SpringArmComponent.TargetArmLength` _springarm) (* ActionValue 30.0)) 100.0 1000.0) _springarm)))

(event `EnhancedInput|/Game/Data/Input/IA_RotateCameraMouse`
  (params (ActionValue :type "Float (double-precision)") (ElapsedSeconds :type "Float (double-precision)") (TriggeredSeconds :type "Float (double-precision)") (InputAction :type "InputAction Object Reference" :default "/Game/Data/Input/IA_RotateCameraMouse.IA_RotateCameraMouse"))
  (bind _defaultsceneroot (`self.DefaultSceneRoot`))
  ; Camera Mouse Rotation
  (:`Triggered`
    (if (`self.CanRotate?`)
      (`SceneComponent.K2_SetWorldRotation` _defaultsceneroot (`KismetMathLibrary.MakeRotator` 0.0 (.pitch (`SceneComponent.RelativeRotation` _defaultsceneroot)) (+ (* ActionValue 1.5) (.yaw (`SceneComponent.RelativeRotation` _defaultsceneroot)))) false false))))

(event `Key|MiddleMouseButton`
  (params (Key :type "Key Structure"))
  (bind _returnvalue (`GameplayStatics.GetPlayerController` 0))
  ; Scroll click enabling rotation and hiding mouse
  (:`Pressed`
    (set `self.CanRotate?` true)
    (`WidgetBlueprintLibrary.SetInputMode_GameOnly` _returnvalue)
    (set `PlayerController.bShowMouseCursor` false _returnvalue))
  (:`Released`
    (set `self.CanRotate?` false)
    (`WidgetBlueprintLibrary.SetInputMode_GameAndUIEx` _returnvalue null "LockInFullscreen")
    (set `PlayerController.bShowMouseCursor` true _returnvalue)))

(event `EnhancedInput|/Game/Data/Input/IA_RotateCameraQE`
  (params (ActionValue :type "Float (double-precision)") (ElapsedSeconds :type "Float (double-precision)") (TriggeredSeconds :type "Float (double-precision)") (InputAction :type "InputAction Object Reference" :default "/Game/Data/Input/IA_RotateCameraQE.IA_RotateCameraQE"))
  (bind _defaultsceneroot (`self.DefaultSceneRoot`))
  ; Camera QE Rotation
  (:`Triggered`
    (if (not (`self.CanRotate?`))
      (`SceneComponent.K2_SetWorldRotation` _defaultsceneroot (`KismetMathLibrary.MakeRotator` 0.0 (.pitch (`SceneComponent.RelativeRotation` _defaultsceneroot)) (+ ActionValue (.yaw (`SceneComponent.RelativeRotation` _defaultsceneroot)))) false false))))

(fn `UserConstructionScript`)