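; Player controller for a tabletop-style (VTT) combat game, handling unit selection, movement and test combat hotkeys, and creating the combat UI.
; Cursor traces drive double-click unit selection, target collection and right-click AI movement with a cursor effect.
; During combat, movement is limited to the active unit and checks its speed.
; Debug keys add targets, roll weapon attacks and damage against them, or end combat through the game mode's combat manager.
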(event `Key|Three`
  (params (Key :type "Key Structure"))
  ; Testowanie
  (:`Pressed`
    (bind _asbp_vttgame_mode (cast `/Game/Blueprints/Core/BP_VTTGameMode` (`GameplayStatics.GetGameMode`)))
    (`/Game/Blueprints/Core/BP_CombatManager.EndCombat` (`/Game/Blueprints/Core/BP_VTTGameMode.CurrentCombatManager` _asbp_vttgame_mode))))

(event `Key|One`
  (params (Key :type "Key Structure"))
  ; Testowanie
  (:`Pressed`
    (bind _asbp_vttunit (cast `/Game/Blueprints/Units/BP_VTTUnit` (`.HitActor` (`GameplayStatics.BreakHitResult` (`self.GetHitResultUnderCursorByChannel` "TraceTypeQuery1")))))
    (`self.SelectingTargets` _asbp_vttunit)))

(event `Key|Two`
  (params (Key :type "Key Structure"))
  (bind _equipedweapon (`/Game/Blueprints/Units/BP_VTTUnit.EquipedWeapon` (`self.SelectedUnit`)))
  ; Testowanie
  (:`Pressed`
    (for _array_element (`self.SelectedTargets`)
      (bind (_charactersheet_charactername _charactersheet_level _charactersheet_classlevels _charactersheet_race _charactersheet_background _charactersheet_alignment _charactersheet_experiencepoints _charactersheet_stats _charactersheet_darkvisiondistance _charactersheet_proficiencybonus _charactersheet_passiveperception _charactersheet_savingthrows _charactersheet_skillproficiencies _charactersheet_weaponproficiencies _charactersheet_armorproficiencies _charactersheet_actions _charactersheet_vitals _charactersheet_resistances _charactersheet_maxspeed _charactersheet_currentspeed _charactersheet_armorclass) (break `DnD_Character_Sheet` (`/Game/Blueprints/Units/BP_VTTUnit.CharacterSheet` _array_element)))
      (bind (_ishit _iscrit _attackroll) (`/Game/Blueprints/Attacks_Spells_Abilities/Items/DA_Weapon.MakeAttackRoll` _equipedweapon _charactersheet_armorclass))
      (if _ishit
        (`KismetSystemLibrary.PrintString` (`KismetStringLibrary.Conv_IntToString` _attackroll))
        (bind _damage (`/Game/Blueprints/Attacks_Spells_Abilities/Items/DA_Weapon.CalculateDamageRoll` _equipedweapon _iscrit))
        (`/Game/Blueprints/Units/BP_VTTUnit.TakeDamage` _array_element _damage)
        (else
          (`KismetSystemLibrary.PrintString` "Miss!!"))))))

(event `EnhancedInput|/Game/Data/Input/IA_Select`
  (params (ActionValue :type Boolean) (ElapsedSeconds :type "Float (double-precision)") (TriggeredSeconds :type "Float (double-precision)") (InputAction :type "InputAction Object Reference" :default "/Game/Data/Input/IA_Select.IA_Select"))
  ; Selecting Unit With Cursor
)

(event `EnhancedInput|/Game/Data/Input/IA_Select_DoubleClick`
  (params (ActionValue :type Boolean) (ElapsedSeconds :type "Float (double-precision)") (TriggeredSeconds :type "Float (double-precision)") (InputAction :type "InputAction Object Reference" :default "/Game/Data/Input/IA_Select_DoubleClick.IA_Select_DoubleClick"))
  ; Selecting Unit With Cursor
  (:`Triggered`
    (bind _asbp_vttunit (cast `/Game/Blueprints/Units/BP_VTTUnit` (`.HitActor` (`GameplayStatics.BreakHitResult` (`self.GetHitResultUnderCursorByChannel` "TraceTypeQuery1")))))
    (`self.SelectingUnit` _asbp_vttunit)))

(event `Key|RightMouseButton`
  (params (Key :type "Key Structure"))
  (bind _selectedunit (`self.SelectedUnit`))
  (bind _selectedunit_2 (`self.SelectedUnit`))
  (bind (_bblockinghit _binitialoverlap _time _distance _location) (`GameplayStatics.BreakHitResult` (`self.GetHitResultUnderCursorByChannel` "TraceTypeQuery2" false)))
  (bind (_charactersheet_charactername _charactersheet_level _charactersheet_classlevels _charactersheet_race _charactersheet_background _charactersheet_alignment _charactersheet_experiencepoints _charactersheet_stats _charactersheet_darkvisiondistance _charactersheet_proficiencybonus _charactersheet_passiveperception _charactersheet_savingthrows _charactersheet_skillproficiencies _charactersheet_weaponproficiencies _charactersheet_armorproficiencies _charactersheet_actions _charactersheet_vitals _charactersheet_resistances _charactersheet_maxspeed _charactersheet_currentspeed) (break `DnD_Character_Sheet` (`/Game/Blueprints/Units/BP_VTTUnit.CharacterSheet` _selectedunit)))
  (:`Pressed`
    ; Checking if combat is active and if it is, checking if selected unit is the one with active turn
    (bind _selectedunit_3 (`self.SelectedUnit`)
      (:`then`
        (bind _asbp_vttgame_mode (cast `/Game/Blueprints/Core/BP_VTTGameMode` (`GameplayStatics.GetGameMode`)))
        (bind _currentcombatmanager (`/Game/Blueprints/Core/BP_VTTGameMode.CurrentCombatManager` _asbp_vttgame_mode))
        (if (`/Game/Blueprints/Core/BP_CombatManager.CombatStateActive` _currentcombatmanager)
          (if (== _selectedunit_3 (`/Game/Blueprints/Core/BP_CombatManager.ActiveUnit` _currentcombatmanager))
            ; Checking what move speed unit has in combat (Experimental)
            (if (>= _charactersheet_currentspeed 0.0)
              (set `/Game/Blueprints/Units/BP_VTTUnit.IsMoving` true _selectedunit)
              ; Moving Unit Out Of Combat (Experimental)
              (`|AIMoveTo` _selectedunit_2 _location null 10.0 :!label _label
                (:`then`
                  (`NiagaraFunctionLibrary.SpawnSystemAtLocation` "/Game/Art/Cursor/FX_Cursor.FX_Cursor" _location))
                (:`OnSuccess`
                  (set `/Game/Blueprints/Units/BP_VTTUnit.IsMoving` false _selectedunit_2)))
              (else
                (`KismetSystemLibrary.PrintString` "Brak ruchu"))))
          (else
            (goto _label))))
      (:`else`))))

(event `self.ReceiveBeginPlay`
  (bind _returnvalue (subsystem `EnhancedInputLocalPlayerSubsystem`))
  (`/Engine/EditorBlueprintResources/StandardMacros.IsValid` _returnvalue
    (:`Is Valid`
      (`EnhancedInputSubsystemInterface.AddMappingContext` _returnvalue "/Game/Data/Input/IMC_Default.IMC_Default" 0 (struct))
      (bind _returnvalue_2 (`|CreateWidget` "/Game/Blueprints/UI/WBP_CombatUI.WBP_CombatUI_C"))
      (`UserWidget.AddToViewport` _returnvalue_2 0))))

(event `self.ReceiveTick`
  (params (DeltaSeconds :type "Float (single-precision)")))

(fn `SelectingTargets`
  (params (SelectedTarget :type "/Game/Blueprints/Units/BP_VTTUnit Object Reference"))
  (`SceneComponent.SetVisibility` (`/Game/Blueprints/Units/BP_VTTUnit.TargetSelectionIndicator` SelectedTarget) true false)
  (`KismetArrayLibrary.Array_Add` (`self.SelectedTargets`) SelectedTarget))

(fn `SelectingUnit`
  (params (SelectedUnit :type "/Game/Blueprints/Units/BP_VTTUnit Object Reference"))
  (bind _selectedunit (`self.SelectedUnit`)
    (:`then`
      (`SceneComponent.SetVisibility` (`/Game/Blueprints/Units/BP_VTTUnit.SelectionIndicator` _selectedunit) false false))
    (:`else`
      _))
  (bind _output_get (set `self.SelectedUnit` SelectedUnit))
  (`SceneComponent.SetVisibility` (`/Game/Blueprints/Units/BP_VTTUnit.SelectionIndicator` _output_get) true false))

(fn `UserConstructionScript`)